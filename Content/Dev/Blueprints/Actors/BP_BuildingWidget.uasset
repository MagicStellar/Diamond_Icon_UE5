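; BP_BuildingWidget is an actor that carries two widget components, a building name label and a floor UI.
; ShowFLoorsUI swaps them, making the floor widget visible and collapsing the name widget.
; Setup that hides the floor UI and binds that event to the W_BuildingUI name button is disconnected, as is FloorUITimeline.
; BeginPlay is empty, so nothing in this graph triggers the swap.
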(event Custom|ShowFLoorsUI
  (Variables|/Script/UMG.Widget|SetVisibility (UserInterface|GetWidget (Variables|Default|GetFloorUI)) "Visible")
  (Variables|/Script/UMG.Widget|SetVisibility (UserInterface|GetWidget (Variables|Default|GetBuildingName)) "Collapsed"))

(event EventBeginPlay)

(event Collision|EventActorBeginOverlap
  (params (OtherActor :type Actor%20Object%20Reference)))

(event EventTick
  (params (DeltaSeconds :type Float%20%28single-precision%29)))

(fn ConstructionScript)