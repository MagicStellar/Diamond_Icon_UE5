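; Main player controller that bootstraps the sky, a building widget actor and the HUD on BeginPlay.
; SpawnMainActors spawns and stores Ultra_Dynamic_Sky and BP_BuildingWidget, then the main HUD widget is added to the viewport.
; Input is set to Game and UI with the HUD focused and the mouse cursor shown.
; An interface function exposes the spawned sky to other objects.
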(event EventBeginPlay
  ;[0.2334 1 0.3969] BeginPlay
  (Utilities|SpawnMainActors
    (:Output
      (bind _returnvalue (UserInterface|CreateWidget "/Game/Dev/UI/UMG/W_MainHUD.W_MainHUD_C" self))
      (Variables|Default|SetW_MainHud _returnvalue)
      (UserInterface|Viewport|AddtoViewport _returnvalue 0)
      (Input|SetInputModeGameandUI self (Variables|Default|GetW_MainHud) "DoNotLock" true false)
      (Variables|Default|SetbShowMouseCursor self true))))

(event EventTick
  (params (DeltaSeconds :type Float%20%28single-precision%29)))

(fn ConstructionScript)

(fn BPIMainControllerGetsky
  (return (Variables|Default|GetAC_Sky)))